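; Actor that shows a random character mesh and sets a material as the CharacterImage of a given card.
; GenerateMesh increments the player character's MeshRenderCount and offsets the actor by a multiple of it, spacing out successive instances.
; It then picks from MeshesArray for the mesh and indexes MaterialsArray for the card image.
; Mesh and image use separate Random evaluations, so they can differ.
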(event Custom|GenerateMesh
  (params (Card :type WBP%20Character%20Card%20Object%20Reference))
  (bind _meshesarray (Variables|Default|GetMeshesArray))
  (bind (_outitem _outindex) (Utilities|Array|Random _meshesarray))
  (bind _asbp_main_character (Utilities|Casting|CastToBP_MainCharacter (Game|Player|GetPlayerPawn 0)))
  (bind _result (Math|Integer|IncrementInt (Variables|/Game/Misc/BP_MainCharacter.BP_MainCharacter_C|GetMeshRenderCount _asbp_main_character))
    (:%20%20
      (Transformation|AddActorWorldOffset (Math|Conversions|ToVector(Float) (* _result 200)))
      (Components|StaticMesh|SetStaticMesh (Variables|Default|GetStaticMesh) _outitem)
      (Class|Image|SetBrushfromMaterial (Variables|/Game/Cards/WBP_CharacterCard.WBP_CharacterCard_C|GetCharacterImage Card) (Utilities|Array|Get(acopy) (Variables|Default|GetMaterialsArray) _outindex)))))

(event EventBeginPlay)

(event Collision|EventActorBeginOverlap
  (params (OtherActor :type Actor%20Object%20Reference)))

(event EventTick
  (params (DeltaSeconds :type Float%20%28single-precision%29)))

(fn ConstructionScript)