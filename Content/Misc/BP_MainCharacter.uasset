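; BP_MainCharacter is the player pawn that sets up the card inventory UI and off-world mesh previews at BeginPlay.
; It creates the main widget, then loops through card slot indices against CardIndexArray and initializes the widget's inventory cards.
; It also spawns BP_CharacterMesh actors far from the origin, offsetting each and pairing its mesh and SceneCapture2D with an indexed render target.
; PopulateUnplayableSlotsWithCards is an empty stub.
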(event Custom|CheckIfRepopulateCards
  (bind _mainwidget (Variables|Default|GetMainWidget))
  (for _index (range 0 4)
    (bind _array_element (Utilities|Array|ForEachLoopwithBreak (Variables|Default|GetCardIndexArray) :!label _label)
      (:LoopBody
        (if (== _array_element _index)
          (goto _label Break)))
      (:Completed
        (Default|InitCard (Utilities|Array|Get(acopy) (Variables|/Game/Main/WBP_MainWidget.WBP_MainWidget_C|GetInventoryCardArray _mainwidget) _index) _mainwidget _index)))))

(event Custom|GenerateRenderers
  (bind _returnvalue (Game|SpawnActorfromClass "/Game/Screenshots/BP_CharacterMesh.BP_CharacterMesh_C" (Math|Transform|MakeTransform "-8099450.000000,311330.000000,4382550.000000") "Undefined" 0 0))
  (CallFunction|GenerateMesh _returnvalue))

(event Custom|GenerateMesh
  (params (CharacterMeshRenderer :type BP%20Character%20Mesh%20Object%20Reference))
  (bind _output_get (Variables|Default|SetCharacter%20Mesh%20Renderer CharacterMeshRenderer))
  (Transformation|AddActorWorldOffset _output_get (Math|Conversions|ToVector(Float) (* (Variables|Default|GetMeshRenderCount) 300)))
  (Components|StaticMesh|SetStaticMesh (Variables|/Game/Screenshots/BP_CharacterMesh.BP_CharacterMesh_C|GetStaticMesh (Variables|Default|GetCharacter%20Mesh%20Renderer)) (Utilities|Array|Get(acopy) (Variables|/Game/Screenshots/BP_CharacterMesh.BP_CharacterMesh_C|GetMeshesArray (Variables|Default|GetCharacter%20Mesh%20Renderer)) (Variables|Default|GetMeshRenderCount)))
  (bind _asbp_main_character (Utilities|Casting|CastToBP_MainCharacter (Game|Player|GetPlayerPawn 0)))
  (Variables|/Script/Engine.SceneCaptureComponent2D|SetTextureTarget (Variables|/Game/Screenshots/BP_CharacterMesh.BP_CharacterMesh_C|GetSceneCaptureComponent2D (Variables|Default|GetCharacter%20Mesh%20Renderer)) (Utilities|Array|Get(acopy) (Variables|BP_MainCharacter_C|GetRenderTargetsArray _asbp_main_character) (Variables|Default|GetMeshRenderCount)))
  (Math|Integer|IncrementInt (Variables|Default|GetMeshRenderCount)
    (:%20%20
      (Utilities|Array|Add (Variables|Default|GetRenderMeshesArray) (Variables|Default|GetCharacter%20Mesh%20Renderer)))))

(event Custom|PopulateUnplayableSlotsWithCards)

(event EventBeginPlay
  (bind _returnvalue (UserInterface|CreateWidget "/Game/Main/WBP_MainWidget.WBP_MainWidget_C"))
  (bind _output_get (Variables|Default|SetMainWidget _returnvalue))
  (UserInterface|Viewport|AddtoViewport _output_get 0)
  (CallFunction|CheckifRepopulateCards)
  (for _index (range 0 3)
    (CallFunction|GenerateRenderers)))

(event Collision|EventActorBeginOverlap
  (params (OtherActor :type Actor%20Object%20Reference)))

(event EventTick
  (params (DeltaSeconds :type Float%20%28single-precision%29)))

(fn ConstructionScript)